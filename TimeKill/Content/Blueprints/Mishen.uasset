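; Mishen is a destructible target actor that loses health when hit by bullets.
; An overlap on its BoxMishen component with a BulletBlueprint destroys the bullet and decrements HPMishen.
; When HPMishen runs out, the target destroys itself and decrements the shared KolvoMishenGI target count stored in GameInstans123.
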(event `self.ReceiveBeginPlay`)

(event `self.BoxMishen.OnComponentBeginOverlap`
  (params (OverlappedComponent :type "PrimitiveComponent Object Reference") (OtherActor :type "Actor Object Reference") (OtherComp :type "PrimitiveComponent Object Reference") (OtherBodyIndex :type Integer) (bFromSweep :type Boolean) (SweepResult :type "HitResult Structure (by ref)"))
  (bind _asbullet_blueprint (cast `/Game/Blueprints/BulletBlueprint` OtherActor))
  (`self.K2_DestroyActor` _asbullet_blueprint)
  (`/Engine/EditorBlueprintResources/StandardMacros.DecrementInt` (`self.HP_mishen`)
    (:`  `
      (if (<= (`self.HP_mishen`) 0)
        (`self.K2_DestroyActor`)
        (bind _asgame_instans_123 (cast `/Game/Blueprints/GameInstans123` (`GameplayStatics.GetGameInstance`)))
        (set `self.kolvo_mishen` (`/Game/Blueprints/GameInstans123.Kolvo_Mishen(GI)` _asgame_instans_123))
        (bind _result (`/Engine/EditorBlueprintResources/StandardMacros.DecrementInt` (`self.kolvo_mishen`))
          (:`  `
            (set `/Game/Blueprints/GameInstans123.Kolvo_Mishen(GI)` _result _asgame_instans_123)))))))

(fn `UserConstructionScript`)