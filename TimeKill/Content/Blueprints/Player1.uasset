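; Player1 is a three-lane shooter pawn or actor that loads bullets into lanes, fires them, then prints victory or defeat from the GameInstance target count.
; BeginPlay passes it to a UI widget, and Upravlenie snaps it to the clamped lane.
; Once started, Tick uses a Delay to stack bullets in the current lane, alongside countdown actors.
; At the bullet limit, Vistrel moves them upward sequentially, advancing when each becomes invalid.
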(event `Spawn_bullets`
  (switch `int` (`self.Position1`)
    (:`0`
      (`self.Levo_spawn_bullets`)
      (`/Engine/EditorBlueprintResources/StandardMacros.IncrementInt` (`self.Kolvo_puli_Levo`)))
    (:`1`
      (`self.Center_spawn_bullets`)
      (`/Engine/EditorBlueprintResources/StandardMacros.IncrementInt` (`self.Kolvo_puli_centr`)))
    (:`2`
      (`self.Pravo_spawn_bullets`)
      (`/Engine/EditorBlueprintResources/StandardMacros.IncrementInt` (`self.Kolvo_puli_Pravo`)))))

(event `Stawn_Otschet`
  (`/Engine/EditorBlueprintResources/StandardMacros.DoOnce` false
    (:`Completed`
      (bind _returnvalue (`|SpawnActorFromClass` "/Game/Blueprints/Otschet.Otschet_C" (`KismetMathLibrary.MakeTransform` (0.0 10.0 0.0) (struct)) "Undefined" "OverrideRootScale"))
      (set `self.Otschet` _returnvalue))))

(event `Upravlenie`
  (`self.Check_Upravlenie_LevoPravo`)
  (switch `int` (`self.Position1`)
    (:`0`
      (`self.K2_SetActorLocation` (-240.0 1.0 -540.0)))
    (:`1`
      (`self.K2_SetActorLocation` (0.0 1.0 -540.0)))
    (:`2`
      (`self.K2_SetActorLocation` (240.0 1.0 -540.0)))))

(event `self.ReceiveBeginPlay`
  (bind _returnvalue (`|CreateWidget` "/Game/Blueprints/WidgetBlueprint.WidgetBlueprint_C" (`GameplayStatics.GetPlayerController` 0)))
  (`UserWidget.AddToViewport` _returnvalue 0)
  (set `/Game/Blueprints/WidgetBlueprint.YaHzPlayer1` self _returnvalue))

(event `self.ReceiveTick`
  (params (DeltaSeconds :type "Float (single-precision)"))
  (bind _returnvalue (`KismetMathLibrary.MakeTransform` (0.0 10.0 0.0) (struct)))
  (bind _letyshaya_pulya (`self.Letyshaya_pulya`))
  (bind _pulik_v_igre (`self.Pulik_v_igre`))
  (if (`self.Start_igri`)
    (if (`self.Cifri`)
      (`|SpawnActorFromClass` "/Game/Blueprints/Cifri.Cifri_C" _returnvalue "Undefined" "OverrideRootScale")
      (set `self.Cifri` false)
      (else
        (`self.K2_DestroyActor` (stale _returnvalue_2))
        (`self.Stawn_Otschet`)
        (if (< (+ (`self.Kolvo_puli_Levo`) (`self.Kolvo_puli_centr`) (`self.Kolvo_puli_Pravo`)) _pulik_v_igre)
          (`KismetSystemLibrary.Delay` 1.0)
          (bind _result (`/Engine/EditorBlueprintResources/StandardMacros.IncrementInt` (`self.Timer`))
            (:`  `
              (set `self.Timer` _result)
              (`self.Spawn_bullets`)))
          (elif (`self.Nalicie_Otscheta`)
            (`self.K2_DestroyActor` (`self.Otschet`))
            (set `self.Nalicie_Otscheta` false)
            (elif (< _letyshaya_pulya _pulik_v_igre)
              (bind _item (`KismetArrayLibrary.Array_Get` (`self.Bull_na_karte`) (stale _result_2)))
              (`self.Vistrel` _item)
              (if (not (`KismetSystemLibrary.IsValid` _item))
                (bind _result_2 (`/Engine/EditorBlueprintResources/StandardMacros.IncrementInt` _letyshaya_pulya)
                  (:`  `
                    (bind _asgame_instans_123 (cast `/Game/Blueprints/GameInstans123` (`GameplayStatics.GetGameInstance`)))
                    (set `self.Kolvo_mishen` (`/Game/Blueprints/GameInstans123.Kolvo_Mishen(GI)` _asgame_instans_123))
                    (set `/Game/Blueprints/GameInstans123.Kolvo_Mishen(GI)` (`self.kolvo_mishen`) _asgame_instans_123)
                    (if (<= (- (`self.Pulik_v_igre`) (`self.Letyshaya_pulya`)) 0)
                      (if (<= (`self.Kolvo_mishen`) 0)
                        (`KismetSystemLibrary.PrintString` "Pobeda")
                        (else
                          (`KismetSystemLibrary.PrintString` "Porqzhenie"))))))))))))
    (else
      (`/Engine/EditorBlueprintResources/StandardMacros.DoOnce` false
        (:`Completed`
          (bind _returnvalue_2 (`|SpawnActorFromClass` "/Game/Blueprints/Otschet.Otschet_C" _returnvalue "Undefined" "OverrideRootScale")))))))

(fn `Center_spawn_bullets`
  (switch `int` (`self.Kolvo_puli_centr`)
    (:`0`
      (bind _returnvalue (`|SpawnActorFromClass` "/Game/Blueprints/BulletBlueprint.BulletBlueprint_C" (`KismetMathLibrary.MakeTransform` (0.0 10.0 -400.0)) "Undefined" "OverrideRootScale"))
      (bind _output_get (set `self.1Bull_center` _returnvalue))
      (`KismetArrayLibrary.Array_Add` (`self.Bull_na_karte`) _output_get))
    (:`1`
      (`self.K2_SetActorLocation` (`self.1Bull_center`) (-10.0 10.0 -400.0) false false)
      (bind _returnvalue_2 (`|SpawnActorFromClass` "/Game/Blueprints/BulletBlueprint.BulletBlueprint_C" (`KismetMathLibrary.MakeTransform` (10.0 10.0 -400.0)) "Undefined" "OverrideRootScale"))
      (bind _output_get_2 (set `self.2Bull_center` _returnvalue_2))
      (`KismetArrayLibrary.Array_Add` (`self.Bull_na_karte`) _output_get_2))
    (:`2`
      (`self.K2_SetActorLocation` (`self.1Bull_center`) (-20.0 10.0 -400.0) false false)
      (`self.K2_SetActorLocation` (`self.2Bull_center`) (0.0 10.0 -400.0) false false)
      (bind _returnvalue_3 (`|SpawnActorFromClass` "/Game/Blueprints/BulletBlueprint.BulletBlueprint_C" (`KismetMathLibrary.MakeTransform` (20.0 10.0 -400.0)) "Undefined" "OverrideRootScale"))
      (bind _output_get_3 (set `self.3Bull_center` _returnvalue_3))
      (`KismetArrayLibrary.Array_Add` (`self.Bull_na_karte`) _output_get_3))
    (:`3`
      (`self.K2_SetActorLocation` (`self.1Bull_center`) (-30.0 10.0 -400.0) false false)
      (`self.K2_SetActorLocation` (`self.2Bull_center`) (-10.0 10.0 -400.0) false false)
      (`self.K2_SetActorLocation` (`self.3Bull_center`) (10.0 10.0 -400.0) false false)
      (bind _returnvalue_4 (`|SpawnActorFromClass` "/Game/Blueprints/BulletBlueprint.BulletBlueprint_C" (`KismetMathLibrary.MakeTransform` (30.0 10.0 -400.0)) "Undefined" "OverrideRootScale"))
      (bind _output_get_4 (set `self.4Bull_center` _returnvalue_4))
      (`KismetArrayLibrary.Array_Add` (`self.Bull_na_karte`) _output_get_4))
    (:`4`
      (bind _returnvalue_5 (`|SpawnActorFromClass` "/Game/Blueprints/BulletBlueprint.BulletBlueprint_C" (`KismetMathLibrary.MakeTransform` (0.0 10.0 -370.0)) "Undefined" "OverrideRootScale"))
      (bind _output_get_5 (set `self.5Bull_center` _returnvalue_5))
      (`KismetArrayLibrary.Array_Add` (`self.Bull_na_karte`) _output_get_5))
    (:`5`
      (`self.K2_SetActorLocation` (`self.5Bull_center`) (-10.0 10.0 -370.0) false false)
      (bind _returnvalue_6 (`|SpawnActorFromClass` "/Game/Blueprints/BulletBlueprint.BulletBlueprint_C" (`KismetMathLibrary.MakeTransform` (10.0 10.0 -370.0)) "Undefined" "OverrideRootScale"))
      (bind _output_get_6 (set `self.6Bull_center` _returnvalue_6))
      (`KismetArrayLibrary.Array_Add` (`self.Bull_na_karte`) _output_get_6))
    (:`6`
      (`self.K2_SetActorLocation` (`self.5Bull_center`) (-20.0 10.0 -370.0) false false)
      (`self.K2_SetActorLocation` (`self.6Bull_center`) (0.0 10.0 -370.0) false false)
      (bind _returnvalue_7 (`|SpawnActorFromClass` "/Game/Blueprints/BulletBlueprint.BulletBlueprint_C" (`KismetMathLibrary.MakeTransform` (20.0 10.0 -370.0)) "Undefined" "OverrideRootScale"))
      (bind _output_get_7 (set `self.7Bull_center` _returnvalue_7))
      (`KismetArrayLibrary.Array_Add` (`self.Bull_na_karte`) _output_get_7))
    (:`7`
      (`self.K2_SetActorLocation` (`self.5Bull_center`) (-30.0 10.0 -370.0) false false)
      (`self.K2_SetActorLocation` (`self.6Bull_center`) (-10.0 10.0 -370.0) false false)
      (`self.K2_SetActorLocation` (`self.7Bull_center`) (10.0 10.0 -370.0) false false)
      (bind _returnvalue_8 (`|SpawnActorFromClass` "/Game/Blueprints/BulletBlueprint.BulletBlueprint_C" (`KismetMathLibrary.MakeTransform` (30.0 10.0 -370.0)) "Undefined" "OverrideRootScale"))
      (bind _output_get_8 (set `self.8Bull_center` _returnvalue_8))
      (`KismetArrayLibrary.Array_Add` (`self.Bull_na_karte`) _output_get_8))))

(fn `Check_Upravlenie_LevoPravo`
  (bind _position1 (`self.Position1`))
  (if (<= _position1 0)
    (set `self.Position1` 0)
    (elif (>= _position1 2)
      (set `self.Position1` 2))))

(fn `Levo_spawn_bullets`
  (bind _1bull_levo (`self.1Bull_levo`))
  (bind _2bull_levo (`self.2Bull_levo`))
  (bind _5bull_levo (`self.5Bull_levo`))
  (bind _6bull_levo (`self.6Bull_levo`))
  (switch `int` (`self.Kolvo_puli_Levo`)
    (:`0`
      (bind _returnvalue (`|SpawnActorFromClass` "/Game/Blueprints/BulletBlueprint.BulletBlueprint_C" (`KismetMathLibrary.MakeTransform` (-240.0 10.0 -400.0)) "Undefined" "OverrideRootScale"))
      (bind _output_get (set `self.1Bull_levo` _returnvalue))
      (`KismetArrayLibrary.Array_Add` (`self.Bull_na_karte`) _output_get))
    (:`1`
      (`self.K2_SetActorLocation` _1bull_levo (-250.0 10.0 -400.0) false false)
      (bind _returnvalue_2 (`|SpawnActorFromClass` "/Game/Blueprints/BulletBlueprint.BulletBlueprint_C" (`KismetMathLibrary.MakeTransform` (-230.0 10.0 -400.0)) "Undefined" "OverrideRootScale"))
      (bind _output_get_2 (set `self.2Bull_levo` _returnvalue_2))
      (`KismetArrayLibrary.Array_Add` (`self.Bull_na_karte`) _output_get_2))
    (:`2`
      (`self.K2_SetActorLocation` _1bull_levo (-260.0 10.0 -400.0) false false)
      (`self.K2_SetActorLocation` _2bull_levo (-240.0 10.0 -400.0) false false)
      (bind _returnvalue_3 (`|SpawnActorFromClass` "/Game/Blueprints/BulletBlueprint.BulletBlueprint_C" (`KismetMathLibrary.MakeTransform` (-220.0 10.0 -400.0)) "Undefined" "OverrideRootScale"))
      (bind _output_get_3 (set `self.3Bull_levo` _returnvalue_3))
      (`KismetArrayLibrary.Array_Add` (`self.Bull_na_karte`) _output_get_3))
    (:`3`
      (`self.K2_SetActorLocation` _1bull_levo (-270.0 10.0 -400.0) false false)
      (`self.K2_SetActorLocation` _2bull_levo (-250.0 10.0 -400.0) false false)
      (`self.K2_SetActorLocation` (`self.3Bull_levo`) (-230.0 10.0 -400.0) false false)
      (bind _returnvalue_4 (`|SpawnActorFromClass` "/Game/Blueprints/BulletBlueprint.BulletBlueprint_C" (`KismetMathLibrary.MakeTransform` (-210.0 10.0 -400.0)) "Undefined" "OverrideRootScale"))
      (bind _output_get_4 (set `self.4Bull_levo` _returnvalue_4))
      (`KismetArrayLibrary.Array_Add` (`self.Bull_na_karte`) _output_get_4))
    (:`4`
      (bind _returnvalue_5 (`|SpawnActorFromClass` "/Game/Blueprints/BulletBlueprint.BulletBlueprint_C" (`KismetMathLibrary.MakeTransform` (-240.0 10.0 -370.0)) "Undefined" "OverrideRootScale"))
      (bind _output_get_5 (set `self.5Bull_levo` _returnvalue_5))
      (`KismetArrayLibrary.Array_Add` (`self.Bull_na_karte`) _output_get_5))
    (:`5`
      (`self.K2_SetActorLocation` _5bull_levo (-250.0 10.0 -370.0) false false)
      (bind _returnvalue_6 (`|SpawnActorFromClass` "/Game/Blueprints/BulletBlueprint.BulletBlueprint_C" (`KismetMathLibrary.MakeTransform` (-230.0 10.0 -370.0)) "Undefined" "OverrideRootScale"))
      (bind _output_get_6 (set `self.6Bull_levo` _returnvalue_6))
      (`KismetArrayLibrary.Array_Add` (`self.Bull_na_karte`) _output_get_6))
    (:`6`
      (`self.K2_SetActorLocation` _5bull_levo (-260.0 10.0 -370.0) false false)
      (`self.K2_SetActorLocation` _6bull_levo (-240.0 10.0 -370.0) false false)
      (bind _returnvalue_7 (`|SpawnActorFromClass` "/Game/Blueprints/BulletBlueprint.BulletBlueprint_C" (`KismetMathLibrary.MakeTransform` (-220.0 10.0 -370.0)) "Undefined" "OverrideRootScale"))
      (bind _output_get_7 (set `self.7Bull_levo` _returnvalue_7))
      (`KismetArrayLibrary.Array_Add` (`self.Bull_na_karte`) _output_get_7))
    (:`7`
      (`self.K2_SetActorLocation` _5bull_levo (-270.0 10.0 -370.0) false false)
      (`self.K2_SetActorLocation` _6bull_levo (-250.0 10.0 -370.0) false false)
      (`self.K2_SetActorLocation` (`self.7Bull_levo`) (-230.0 10.0 -370.0) false false)
      (bind _returnvalue_8 (`|SpawnActorFromClass` "/Game/Blueprints/BulletBlueprint.BulletBlueprint_C" (`KismetMathLibrary.MakeTransform` (-210.0 10.0 -370.0)) "Undefined" "OverrideRootScale"))
      (bind _output_get_8 (set `self.8Bull_levo` _returnvalue_8))
      (`KismetArrayLibrary.Array_Add` (`self.Bull_na_karte`) _output_get_8))))

(fn `NewFunction_0`
  (returns (kovo_mishen :type Integer))
  (return 0))

(fn `Pravo_spawn_bullets`
  (bind _5bull_pravo (`self.5Bull_pravo`))
  (bind _6bull_pravo (`self.6Bull_pravo`))
  (bind _1bull_pravo (`self.1Bull_pravo`))
  (bind _2bull_pravo (`self.2Bull_pravo`))
  (switch `int` (`self.Kolvo_puli_Pravo`)
    (:`0`
      (bind _returnvalue (`|SpawnActorFromClass` "/Game/Blueprints/BulletBlueprint.BulletBlueprint_C" (`KismetMathLibrary.MakeTransform` (240.0 10.0 -400.0)) "Undefined" "OverrideRootScale"))
      (bind _output_get (set `self.1Bull_pravo` _returnvalue))
      (`KismetArrayLibrary.Array_Add` (`self.Bull_na_karte`) _output_get))
    (:`1`
      (`self.K2_SetActorLocation` _1bull_pravo (230.0 10.0 -400.0) false false)
      (bind _returnvalue_2 (`|SpawnActorFromClass` "/Game/Blueprints/BulletBlueprint.BulletBlueprint_C" (`KismetMathLibrary.MakeTransform` (250.0 10.0 -400.0)) "Undefined" "OverrideRootScale"))
      (bind _output_get_2 (set `self.2Bull_pravo` _returnvalue_2))
      (`KismetArrayLibrary.Array_Add` (`self.Bull_na_karte`) _output_get_2))
    (:`2`
      (`self.K2_SetActorLocation` _1bull_pravo (220.0 10.0 -400.0) false false)
      (`self.K2_SetActorLocation` _2bull_pravo (240.0 10.0 -400.0) false false)
      (bind _returnvalue_3 (`|SpawnActorFromClass` "/Game/Blueprints/BulletBlueprint.BulletBlueprint_C" (`KismetMathLibrary.MakeTransform` (260.0 10.0 -400.0)) "Undefined" "OverrideRootScale"))
      (bind _output_get_3 (set `self.3Bull_pravo` _returnvalue_3))
      (`KismetArrayLibrary.Array_Add` (`self.Bull_na_karte`) _output_get_3))
    (:`3`
      (`self.K2_SetActorLocation` _1bull_pravo (210.0 10.0 -400.0) false false)
      (`self.K2_SetActorLocation` _2bull_pravo (230.0 10.0 -400.0) false false)
      (`self.K2_SetActorLocation` (`self.3Bull_pravo`) (250.0 10.0 -400.0) false false)
      (bind _returnvalue_4 (`|SpawnActorFromClass` "/Game/Blueprints/BulletBlueprint.BulletBlueprint_C" (`KismetMathLibrary.MakeTransform` (270.0 10.0 -400.0)) "Undefined" "OverrideRootScale"))
      (bind _output_get_4 (set `self.4Bull_pravo` _returnvalue_4))
      (`KismetArrayLibrary.Array_Add` (`self.Bull_na_karte`) _output_get_4))
    (:`4`
      (bind _returnvalue_5 (`|SpawnActorFromClass` "/Game/Blueprints/BulletBlueprint.BulletBlueprint_C" (`KismetMathLibrary.MakeTransform` (240.0 10.0 -370.0)) "Undefined" "OverrideRootScale"))
      (bind _output_get_5 (set `self.5Bull_pravo` _returnvalue_5))
      (`KismetArrayLibrary.Array_Add` (`self.Bull_na_karte`) _output_get_5))
    (:`5`
      (`self.K2_SetActorLocation` _5bull_pravo (230.0 10.0 -370.0) false false)
      (bind _returnvalue_6 (`|SpawnActorFromClass` "/Game/Blueprints/BulletBlueprint.BulletBlueprint_C" (`KismetMathLibrary.MakeTransform` (250.0 10.0 -370.0)) "Undefined" "OverrideRootScale"))
      (bind _output_get_6 (set `self.6Bull_pravo` _returnvalue_6))
      (`KismetArrayLibrary.Array_Add` (`self.Bull_na_karte`) _output_get_6))
    (:`6`
      (`self.K2_SetActorLocation` _5bull_pravo (220.0 10.0 -370.0) false false)
      (`self.K2_SetActorLocation` _6bull_pravo (240.0 10.0 -370.0) false false)
      (bind _returnvalue_7 (`|SpawnActorFromClass` "/Game/Blueprints/BulletBlueprint.BulletBlueprint_C" (`KismetMathLibrary.MakeTransform` (260.0 10.0 -370.0)) "Undefined" "OverrideRootScale"))
      (bind _output_get_7 (set `self.7Bull_pravo` _returnvalue_7))
      (`KismetArrayLibrary.Array_Add` (`self.Bull_na_karte`) _output_get_7))
    (:`7`
      (`self.K2_SetActorLocation` _5bull_pravo (210.0 10.0 -370.0) false false)
      (`self.K2_SetActorLocation` _6bull_pravo (230.0 10.0 -370.0) false false)
      (`self.K2_SetActorLocation` (`self.7Bull_pravo`) (250.0 10.0 -370.0) false false)
      (bind _returnvalue_8 (`|SpawnActorFromClass` "/Game/Blueprints/BulletBlueprint.BulletBlueprint_C" (`KismetMathLibrary.MakeTransform` (270.0 10.0 -370.0)) "Undefined" "OverrideRootScale"))
      (bind _output_get_8 (set `self.8Bull_pravo` _returnvalue_8))
      (`KismetArrayLibrary.Array_Add` (`self.Bull_na_karte`) _output_get_8))))

(fn `UserConstructionScript`)

(fn `Vistrel`
  (params (Bullet :type "/Game/Blueprints/BulletBlueprint Object Reference"))
  (if (`KismetSystemLibrary.IsValid` Bullet)
    (`self.K2_SetActorTransform` Bullet (`KismetMathLibrary.MakeTransform` (`KismetMathLibrary.MakeVector` (.x (.location (`self.GetTransform` Bullet))) (.y (.location (`self.GetTransform` Bullet))) (+ (.z (.location (`self.GetTransform` Bullet))) (`self.Skorost_Puli`))) (.rotation (`self.GetTransform` Bullet)) (.scale (`self.GetTransform` Bullet))) false false)))